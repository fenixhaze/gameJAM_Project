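; GameplayAbility is a base ability Blueprint that exposes activate and deactivate events, with Jaguar as the only handled ability type.
; On BeginPlay it caches the player character and its ABP_Manny animation instance.
; Both events switch on AbilityType and cast self to the matching child class, GameplayAbility_Jaguar, to call its own activate or deactivate function, rather than using overrides.
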(event Custom|ActivateAbility
  (switch Utilities|FlowControl|Switch|SwitchonGameplayAbilityType (Variables|Default|GetAbilityType)
    (:NewEnumerator0
      (bind _asgameplay_ability_jaguar (Utilities|Casting|CastToGameplayAbility_Jaguar self))
      (Default|ActivateJaguarAbility _asgameplay_ability_jaguar))))

(event Custom|DeactiveAbility
  (switch Utilities|FlowControl|Switch|SwitchonGameplayAbilityType (Variables|Default|GetAbilityType)
    (:NewEnumerator0
      (bind _asgameplay_ability_jaguar (Utilities|Casting|CastToGameplayAbility_Jaguar self))
      (Default|DeactivateJaguarAbility _asgameplay_ability_jaguar))))

(event EventBeginPlay
  (References|CharacterRef)
  (References|ABPCharacterRef))

(fn ConstructionScript)

(fn CharacterRef
  (Variables|Default|SetTopDownCaracterReference (Game|GetPlayerCharacter 0)))

(fn ABPCharacterRef
  (bind _asabp_manny (Utilities|Casting|CastToABP_Manny (Components|SkeletalMesh|GetAnimInstance (Variables|/Script/Engine.Character|GetMesh (Game|GetPlayerCharacter 0)))))
  (Variables|References|SetABPMannyReference _asabp_manny))